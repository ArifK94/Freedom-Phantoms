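; Mission select laptop prop that opens the MissionSelection UI when the player interacts with it.
; Overlapping its box registers the laptop as the CustomPlayerController's focused interactable actor.
; On use, it creates the widget, adds it to the viewport, shows the mouse cursor and switches to UI-only input.
; Helper functions supply the interaction message and the display name of the key bound to UseInteractable.
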(event OnComponentBeginOverlap(Box)
  (params (OverlappedComponent :type Primitive%20Component%20Object%20Reference) (OtherActor :type Actor%20Object%20Reference) (OtherComp :type Primitive%20Component%20Object%20Reference) (OtherBodyIndex :type Integer) (bFromSweep :type Boolean) (SweepResult :type Hit%20Result%20Structure%20%28by%20ref%29))
  (if (== OtherActor (Game|GetPlayerCharacter 0))
    (bind _ascustom_player_controller (Utilities|Casting|CastToCustomPlayerController (Game|GetPlayerController 0)))
    (Variables|/Script/FreedomFighters.CustomPlayerController|SetFocusedInteractableActor _ascustom_player_controller self)))

(event EventOnUseInteraction
  (bind _returnvalue (Game|GetPlayerController 0))
  (bind _returnvalue_2 (UserInterface|CreateWidget "/Game/Blueprints/UI/Menu/MissionSelection_UMG.MissionSelection_UMG_C"))
  (UserInterface|Viewport|AddtoViewport _returnvalue_2 0)
  (Variables|/Script/Engine.PlayerController|SetbShowMouseCursor _returnvalue true)
  (Input|SetInputModeUIOnly _returnvalue _returnvalue_2 "DoNotLock"))

(fn ConstructionScript)

(fn GetKeyDisplayName
  (return (Utilities|String|ToString(Text) (Class|KismetInputLibrary|KeyGetDisplayName (.key (Utilities|Array|Get(acopy) (Class|InputSettings|GetActionMappingbyName (Class|InputSettings|GetInputSettings) "UseInteractable")))))))

(fn OnInteractionFound
  (return (Variables|Default|GetActionMessage)))