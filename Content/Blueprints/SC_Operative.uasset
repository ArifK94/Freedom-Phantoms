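; Shooter operative character Blueprint that sets up its HUD and tracks cover state.
; On BeginPlay it creates crosshair, weapon ammo and blood blur widgets; each Tick maps velocity to crosshair spread without clamping.
; Cover events store availability, rotation and high/low flags, and cancel cover-taking when none is available.
; The construction script slaves the separate Head mesh to the body's pose via Master Pose Component.
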(event EventBeginPlay
  (Utilities|FlowControl|Sequence
    (:then_0
      (bind _returnvalue (UserInterface|CreateWidget "/Game/Blueprints/UI/WBCrosshair.WBCrosshair_C"))
      (bind _output_get (Variables|Default|SetCrosshair _returnvalue))
      (UserInterface|Viewport|AddtoViewport _output_get 0))
    (:then_1
      (bind _returnvalue_2 (UserInterface|CreateWidget "/Game/Blueprints/UI/WeaponAmmo_WP.WeaponAmmo_WP_C"))
      (UserInterface|Viewport|AddtoViewport _returnvalue_2 0))
    (:then_2
      (bind _returnvalue_3 (UserInterface|CreateWidget "/Game/Blueprints/UI/BloodBlur.BloodBlur_C"))
      (UserInterface|Viewport|AddtoViewport _returnvalue_3 0))))

(event EventIsCoverAvailable
  (params (IsCoverAvailable :type Boolean) (CoverRotation :type Rotator :default "0, 0, 0") (IsHigh :type Boolean) (IsLow :type Boolean))
  ;[1 1 1] Cover Events
  (bind _output_get (Variables|Default|SetcanTakeCover IsCoverAvailable))
  (Variables|Default|SetCoverRotation CoverRotation)
  (Variables|Default|SetisCoveringHigh IsHigh)
  (Variables|Default|SetisCoveringLow IsLow)
  (if (not _output_get)
    (Variables|Default|SetisTakingCover false)))

(event EventTick
  (params (DeltaSeconds :type Float%20%28single-precision%29))
  (Variables|/Game/Blueprints/UI/WBCrosshair.WBCrosshair_C|Setcrosshair_spread (Variables|Default|GetCrosshair) (Math|Float|MapRangeUnclamped (Math|Vector|VectorLength (Transformation|GetVelocity)) 0.0 2e+02 5.0 8e+01)))

(event EventEndOfCover
  (params (EndOfCoverLeft :type Boolean) (EndOfCoverRight :type Boolean) (isHigh :type Boolean) (IsLow :type Boolean))
  ;[1 1 1] Cover Events
  (Variables|Default|SetisCoveringHigh isHigh)
  (Variables|Default|SetisCoveringLow IsLow))

(fn ConstructionScript
  (Class|SkinnedMeshComponent|SetMasterPoseComponent (Variables|Default|GetHead) (Variables|Character|GetMesh) false))