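; Behavior tree task that moves an AI-controlled BaseCharacter toward a blackboard destination.
; Each AI tick it reads the target and calls MoveToLocation on the controller.
; On a successful request it sets full forward input, sprints when over 200 units away, and finishes without waiting for arrival.
; A failed cast fails the task, while other move results leave it ticking.
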(event EventReceiveTickAI
  (params (OwnerController :type AI%20Controller%20Object%20Reference) (ControlledPawn :type Pawn%20Object%20Reference) (DeltaSeconds :type Float%20%28single-precision%29))
  (Variables|Default|SetTargetLocation (Class|BTFunctionLibrary|GetBlackboardValueasVector (Variables|Default|GetBB_TargetDestination)))
  (Variables|Default|SetOwningController OwnerController)
  (bind _asbase_character (Utilities|Casting|CastToBaseCharacter ControlledPawn)
    (:then
      (Variables|Default|SetOwningCharacter _asbase_character)
      (bind _returnvalue (AI|Navigation|MovetoLocation (Variables|Default|GetOwningController) (Variables|Default|GetTargetLocation) (Variables|Default|GetAcceptanceRadius) true true false true 0))
      (switch Utilities|FlowControl|Switch|SwitchonEPathFollowingRequestResult _returnvalue
        (:RequestSuccessful
          (Variables|/Script/FreedomFighters.BaseCharacter|SetForwardInputValue (Variables|Default|GetOwningCharacter) 1.0)
          (if (> (Math|Vector|Distance(Vector) (Transformation|GetActorLocation (Variables|Default|GetOwningCharacter)) (Variables|Default|GetTargetLocation)) 2e+02)
            (Class|BaseCharacter|BeginSprint (Variables|Default|GetOwningCharacter))
            (else
              (Class|BaseCharacter|EndSprint (Variables|Default|GetOwningCharacter))))
          (AI|BehaviorTree|FinishExecute true))))
    (:CastFailed
      (AI|BehaviorTree|FinishExecute false))))