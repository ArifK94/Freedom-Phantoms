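; Behavior tree service that picks the nearest living hostile CombatCharacter as the AI's target.
; Each tick it scans every CombatCharacter in the world, filtering out friendlies and those without health, then keeps the closest by distance.
; It calls TargetFound on the controlled character whenever a closer candidate turns up and writes the result, or None, to the TargetKey blackboard entry.
; Sight perception is not used; an unconnected perception query remains in the graph.
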(event EventReceiveTickAI
  (params (OwnerController :type AI%20Controller%20Object%20Reference) (ControlledPawn :type Pawn%20Object%20Reference) (DeltaSeconds :type Float%20%28single-precision%29))
  (Variables|Default|SetControlledPawn ControlledPawn)
  (Variables|Default|SetBestTargetActor 0)
  (Variables|Default|SetNearestTargetDistance 1e+08)
  (bind _outactors (Actor|GetAllActorsOfClass "/Script/FreedomFighters.CombatCharacter"))
  (for _array_element _outactors
    (if (and (not (Class|HealthComponent|IsFriendly _array_element (Variables|Default|GetControlledPawn))) (> (Variables|/Script/FreedomFighters.HealthComponent|GetHealth (Actor|GetComponentbyClass _array_element "/Script/FreedomFighters.HealthComponent")) 0.0))
      (if (< (Math|Vector|VectorLength (- (Transformation|GetActorLocation (Variables|Default|GetControlledPawn)) (Transformation|GetActorLocation _array_element))) (Variables|Default|GetNearestTargetDistance))
        (Variables|Default|SetNearestTargetDistance (Math|Vector|VectorLength (- (Transformation|GetActorLocation (Variables|Default|GetControlledPawn)) (Transformation|GetActorLocation _array_element))))
        (Variables|Default|SetBestTargetActor _array_element)
        (bind _ascombat_character (Utilities|Casting|CastToCombatCharacter (Variables|Default|GetControlledPawn)))
        (Class|CombatCharacter|TargetFound _ascombat_character))))
  (Class|BTFunctionLibrary|SetBlackboardValueasObject (Variables|Default|GetTargetKey) (Variables|Default|GetBestTargetActor)))