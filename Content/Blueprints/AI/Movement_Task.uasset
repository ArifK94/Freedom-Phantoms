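; Behavior tree task that moves an AI-controlled BaseCharacter toward a Blackboard destination, sprinting when the target is far away.
; On AI tick it reads the destination vector, casts the pawn and issues MoveToLocation through the controller.
; A distance check starts or ends sprinting, then the task finishes successfully without waiting for arrival.
; It reports failure if the pawn is not a BaseCharacter.
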(event EventReceiveTickAI
  (params (OwnerController :type AI%20Controller%20Object%20Reference) (ControlledPawn :type Pawn%20Object%20Reference) (DeltaSeconds :type Float%20%28single-precision%29))
  (Variables|Default|SetTargetLocation (Class|BTFunctionLibrary|GetBlackboardValueasVector (Variables|Default|GetBB_TargetDestination)))
  (Variables|Default|SetOwningController OwnerController)
  (bind _output_get (Variables|Default|SetControlledPawn ControlledPawn))
  (bind _asbase_character (Utilities|Casting|CastToBaseCharacter _output_get)
    (:then
      (Variables|Default|SetOwningCharacter _asbase_character)
      (AI|Navigation|MovetoLocation (Variables|Default|GetOwningController) (Variables|Default|GetTargetLocation) 5e+01 true true false true 0)
      (if (> (Math|Vector|Distance(Vector) (Transformation|GetActorLocation (Variables|Default|GetOwningCharacter)) (Variables|Default|GetTargetLocation)) 2e+02)
        (Class|BaseCharacter|BeginSprint (Variables|Default|GetOwningCharacter))
        (else
          (Class|BaseCharacter|EndSprint (Variables|Default|GetOwningCharacter))))
      (AI|BehaviorTree|FinishExecute true))
    (:CastFailed
      (AI|BehaviorTree|FinishExecute false))))