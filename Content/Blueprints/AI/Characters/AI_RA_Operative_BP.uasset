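; AI character Blueprint for a Russian Airborne operative that randomizes its appearance when play begins.
; A six-way random roll on BeginPlay swaps the Head component's skeletal mesh among five variants, A to E.
; Two rolls also apply red shotgun upper-body and pants materials to the body mesh: head C, and a second head B with an overridden material.
; The construction script is empty.
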(event EventBeginPlay
  (bind _head (Variables|Default|GetHead))
  (switch int (Math|Random|RandomInteger 6)
    (:Default
      (Class|SkinnedMeshComponent|SetSkeletalMesh _head "/Game/Models/Characters/COD/Airborne_Russian/Head/E/Meshes/Russian_Airborne_Head_E.Russian_Airborne_Head_E" true :!label _label))
    (:0
      (Class|SkinnedMeshComponent|SetSkeletalMesh _head "/Game/Models/Characters/COD/Airborne_Russian/Head/A/Mesh/Russian_Airborne_Head_A.Russian_Airborne_Head_A" true))
    (:1
      (Class|SkinnedMeshComponent|SetSkeletalMesh _head "/Game/Models/Characters/COD/Airborne_Russian/Head/B/Meshes/Russian_Airborne_Head_B.Russian_Airborne_Head_B" true))
    (:2
      (Class|SkinnedMeshComponent|SetSkeletalMesh _head "/Game/Models/Characters/COD/Airborne_Russian/Head/C/Meshes/Russian_Airborne_Head_C.Russian_Airborne_Head_C" true)
      (Rendering|Material|SetMaterial (Variables|Character|GetMesh) 0 "/Game/Models/Characters/COD/Airborne_Russian/Body/Materials/h2_airborne_upperbody_shotgun_red_col_Mat.h2_airborne_upperbody_shotgun_red_col_Mat" :!label _label_2)
      (Rendering|Material|SetMaterial (Variables|Character|GetMesh) 3 "/Game/Models/Characters/COD/Airborne_Russian/Body/Materials/h2_airborne_pants_shotgun_red_col_Mat.h2_airborne_pants_shotgun_red_col_Mat"))
    (:3
      (Class|SkinnedMeshComponent|SetSkeletalMesh _head "/Game/Models/Characters/COD/Airborne_Russian/Head/D/Meshes/Russian_Airborne_Head_D.Russian_Airborne_Head_D" true))
    (:4
      (goto _label))
    (:5
      (Class|SkinnedMeshComponent|SetSkeletalMesh _head "/Game/Models/Characters/COD/Airborne_Russian/Head/B/Meshes/Russian_Airborne_Head_B.Russian_Airborne_Head_B" true)
      (Rendering|Material|SetMaterial (Variables|Default|GetHead) 2 "/Game/Models/Characters/COD/Airborne_Russian/Body/Materials/h2_airborne_head_b_col_Mat.h2_airborne_head_b_col_Mat")
      (goto _label_2))))

(fn ConstructionScript)