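; SC helmet accessory Blueprint that gives itself and its attached goggles a random color variant.
; On BeginPlay it casts the Goggles child actor to Goggle and stores the reference.
; It then randomly picks a green or grey shadow material and applies it to both the helmet mesh and the goggle mesh so they match.
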(event EventBeginPlay
  (bind _mesh (Variables|Character|GetMesh))
  (bind _asgoggle (Utilities|Casting|CastToGoggle (Variables|/Script/Engine.ChildActorComponent|GetChildActor (Variables|Default|GetGoggles))))
  (Variables|Default|SetGoggleObj _asgoggle)
  (switch int (Math|Random|RandomInteger 2)
    (:Default
      (Rendering|Material|SetMaterial _mesh 0 "/Game/Models/Characters/COD/ShadowCompany/Helmet/helmet_shadow_grey.helmet_shadow_grey" :!label _label)
      (Rendering|Material|SetMaterial (Variables|/Script/FreedomFighters.Goggle|GetMesh (Variables|Default|GetGoggleObj)) 0 "/Game/Models/Characters/COD/ShadowCompany/Helmet/helmet_shadow_grey.helmet_shadow_grey"))
    (:0
      (Rendering|Material|SetMaterial _mesh 0 "/Game/Models/Characters/COD/ShadowCompany/Helmet/helmet_shadow_green.helmet_shadow_green")
      (Rendering|Material|SetMaterial (Variables|/Script/FreedomFighters.Goggle|GetMesh (Variables|Default|GetGoggleObj)) 0 "/Game/Models/Characters/COD/ShadowCompany/Helmet/helmet_shadow_green.helmet_shadow_green"))
    (:1
      (goto _label))))

(fn ConstructionScript)