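; SC_NVG_BP is a night vision goggle Blueprint that switches on a post-process vision effect behind a screen fade.
; On BeginPlay it disables VisionPPComp, adds an NVG_QuickFade widget to the viewport, then enables the component after a short delay.
; A mirrored fade-and-disable sequence for switching the effect off is present but unconnected, so it never runs.
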(event EventBeginPlay
  (Variables|/Script/Engine.PostProcessComponent|SetbEnabled (Variables|Default|GetVisionPPComp) false)
  (bind _returnvalue (UserInterface|CreateWidget "/Game/OutlastCameraFiles/NVG_QuickFade.NVG_QuickFade_C"))
  (UserInterface|Viewport|AddtoViewport _returnvalue 0)
  (Utilities|FlowControl|Delay 0.5)
  (Variables|/Script/Engine.PostProcessComponent|SetbEnabled (Variables|Default|GetVisionPPComp) true)
  (Utilities|FlowControl|Delay 1.0))

(fn ConstructionScript)