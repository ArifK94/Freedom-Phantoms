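; M870 shotgun Blueprint that fills its extra ammo holder with visible cartridge actors when play begins.
; BeginPlay scans the socket names on ExtraAmmoHolder for those containing "cartridge".
; For each match it spawns a WeaponClip actor owned by the weapon and snaps it to that socket, so socket naming determines the shell count and placement.
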(event EventBeginPlay
  (for _array_element (Transformation|GetAllSocketNames (Variables|Default|GetExtra_Ammo_Holder))
    (if (Utilities|String|Contains (Utilities|String|ToString(Name) _array_element) "cartridge")
      (bind _returnvalue (Game|SpawnActorfromClass (Variables|Default|GetweaponClip) (Math|Conversions|ToTransform(Vector) (Math|Vector|VectorZero)) "AlwaysSpawn" self 0))
      (Transformation|AttachComponentToComponent _returnvalue (Variables|Default|GetExtra_Ammo_Holder) (Utilities|String|StringToName (Utilities|String|ToString(Name) _array_element)) "SnapToTarget" "SnapToTarget" "KeepRelative" true))))

(fn ConstructionScript)