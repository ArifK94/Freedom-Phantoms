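; Vehicle path actor that holds a spline component defining a route, with visual markers for its points.
; The construction script walks the spline points and adds an arrow and a text label showing the index at each point's world location.
; The labels are enlarged and hidden in game, and the arrows are only positioned, not aligned to the spline.
; The event graph has no active logic.
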(event EventBeginPlay)

(event Collision|EventActorBeginOverlap
  (params (OtherActor :type Actor%20Object%20Reference)))

(event EventTick
  (params (DeltaSeconds :type Float%20%28single-precision%29)))

(fn ConstructionScript
  (for _index (range 0 (Spline|GetNumberOfSplinePoints (Variables|Default|GetSplinePathComp)))
    (bind _returnvalue (AddComponent|AddArrowComponent false))
    (Transformation|SetWorldLocation _returnvalue (Spline|GetLocationatSplinePoint (Variables|Default|GetSplinePathComp) _index "World") false false)
    (bind _returnvalue_2 (AddComponent|AddTextRenderComponent false))
    (Rendering|Components|TextRender|SetText _returnvalue_2 (Utilities|Text|ToText(Integer) _index))
    (Development|SetHiddeninGame _returnvalue_2 true false)
    (Rendering|Components|TextRender|SetWorldSize _returnvalue_2 1e+02)
    (Transformation|SetWorldLocation _returnvalue_2 (Spline|GetLocationatSplinePoint (Variables|Default|GetSplinePathComp) _index "World") false false)))