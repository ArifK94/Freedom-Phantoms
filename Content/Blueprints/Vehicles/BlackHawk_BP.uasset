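; Black Hawk helicopter actor that flies along a spline on an assigned VehiclePath actor, starting on BeginPlay.
; A timeline, with play rate set from Duration and start time from StartOffset, drives an alpha across the spline length.
; Each update snaps the helicopter to the world location and rotation at that distance, and nothing moves if no valid path is set.
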(event Custom|FollowPath
  (Utilities|IsValid (Variables|Default|GetVehiclePath)
    (:Is%20Valid
      (Components|Timeline|SetPlayRate (Variables|Default|GetPathMover) (/ 1.0 (Variables|Default|GetDuration)))
      (Components|Timeline|SetNewTime (Variables|Default|GetPathMover) (Variables|Default|GetStartOffset))
      (bind _alpha (Timeline|PathMover Play)
        (:Update
          (Variables|Default|SetAlpha _alpha)
          (Transformation|SetActorLocationAndRotation (Spline|GetLocationatDistanceAlongSpline (Variables|/Game/Blueprints/Vehicles/VehiclePath.VehiclePath_C|GetUsefulSpline (Variables|Default|GetVehiclePath)) (Math|Float|Lerp 0.0 (Spline|GetSplineLength (Variables|/Game/Blueprints/Vehicles/VehiclePath.VehiclePath_C|GetUsefulSpline (Variables|Default|GetVehiclePath))) (Variables|Default|GetAlpha)) "World") (Spline|GetRotationatDistanceAlongSpline (Variables|/Game/Blueprints/Vehicles/VehiclePath.VehiclePath_C|GetUsefulSpline (Variables|Default|GetVehiclePath)) (Math|Float|Lerp 0.0 (Spline|GetSplineLength (Variables|/Game/Blueprints/Vehicles/VehiclePath.VehiclePath_C|GetUsefulSpline (Variables|Default|GetVehiclePath))) (Variables|Default|GetAlpha)) "World")))))))

(event EventBeginPlay
  (CallFunction|FollowPath))

(fn ConstructionScript)