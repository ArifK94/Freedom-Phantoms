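; Interactable command table prop that opens the mission selection screen.
; It implements interaction functions that always allow interaction and return an action message when found, with an empty key display name.
; Pickup creates the MissionSelection_UMG widget, adds it to the viewport, shows the mouse cursor and switches the player controller to UI-only input focused on that widget.
; The use interaction is a stub that returns false.
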(fn ConstructionScript)

(fn CanInteract
  (params (InPawn :type Pawn%20Object%20Reference) (InController :type Controller%20Object%20Reference))
  (return true))

(fn GetKeyDisplayName
  (return ""))

(fn OnInteractionFound
  (params (InPawn :type Pawn%20Object%20Reference) (InController :type Controller%20Object%20Reference))
  (return (Variables|Default|GetActionMessage)))

(fn OnPickup
  (params (InPawn :type Pawn%20Object%20Reference) (InController :type Controller%20Object%20Reference))
  (bind _asplayer_controller (Utilities|Casting|CastToPlayerController InController))
  (bind _returnvalue (UserInterface|CreateWidget "/Game/_CODFF/Blueprints/UI/Menu/MissionSelection_UMG.MissionSelection_UMG_C"))
  (UserInterface|Viewport|AddtoViewport _returnvalue 0)
  (Variables|/Script/Engine.PlayerController|SetbShowMouseCursor _asplayer_controller true)
  (Input|SetInputModeUIOnly _asplayer_controller _returnvalue "DoNotLock")
  (return 0))

(fn OnUseInteraction
  (params (InPawn :type Pawn%20Object%20Reference) (InController :type Controller%20Object%20Reference))
  (return false))