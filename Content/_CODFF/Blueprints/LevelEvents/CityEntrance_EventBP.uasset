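; Level-event trigger for the city entrance that spawns Airborne AI units once when the player first overlaps its box, then destroys the box.
; For each free StartEventPoint, it spawns a unit 500 units above a random reachable point near the back board of a living entrance truck, randomly picked if both survive.
; Each unit claims its point and, after a one-second delay, moves there as a priority destination.
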(event OnComponentBeginOverlap(Box)
  (params (OverlappedComponent :type Primitive%20Component%20Object%20Reference) (OtherActor :type Actor%20Object%20Reference) (OtherComp :type Primitive%20Component%20Object%20Reference) (OtherBodyIndex :type Integer) (bFromSweep :type Boolean) (SweepResult :type Hit%20Result%20Structure%20%28by%20ref%29))
  (if (CallFunction|IsPlayer OtherActor)
    (Components|DestroyComponent (Variables|Default|GetBox))
    (bind (_positions1 _aimovementcomps1) (CallFunction|MapStartEvent))
    (Variables|Default|SetAIMovement%20Comps%201 _aimovementcomps1)
    (Variables|Default|SetPositions%201 _positions1)
    (Utilities|FlowControl|Delay 1.0)
    (for _index (range 0 (Utilities|Array|Length (Variables|Default|GetAIMovement%20Comps%201)))
      (Utilities|IsValid (Utilities|Array|Get(acopy) (Variables|Default|GetAIMovement%20Comps%201) _index)
        (:Is%20Valid
          (Class|AIMovementComponent|MovetoDestination (Utilities|Array|Get(acopy) (Variables|Default|GetAIMovement%20Comps%201) _index) (Utilities|Array|Get(acopy) (Variables|Default|GetPositions%201) _index) 0.0 "PriorityDestination" true false))))))

(fn ConstructionScript)

(fn IsPlayer
  (params (Actor :type Actor%20Object%20Reference))
  (return (== Actor (Game|GetPlayerCharacter 0))))

(fn GetGroundPoint
  (params (Start :type Vector))
  (return (+ Start "0, 0,500.000000")))

(fn MapStartEvent
  (bind _outactors (Actor|GetAllActorsOfClasswithTag "/Script/Engine.Actor" "StartEventPoint"))
  (for _array_element _outactors
    (bind _outactors_2 (Actor|GetAllActorsOfClasswithTag "/Script/FreedomFighters.LandVehicle" "Entrance_Truck1"))
    (bind _outactors_3 (Actor|GetAllActorsOfClasswithTag "/Script/FreedomFighters.LandVehicle" "Entrance_Truck2"))
    (if (not (Variables|/Script/FreedomFighters.TargetPointComponent|GetIsPointTaken (Actor|GetComponentbyClass _array_element "/Script/FreedomFighters.TargetPointComponent")))
      (if (and (Variables|/Script/FreedomFighters.HealthComponent|GetisAlive (Variables|/Script/FreedomFighters.LandVehicle|GetHealthComp (Utilities|Array|Get(acopy) _outactors_2))) (Variables|/Script/FreedomFighters.HealthComponent|GetisAlive (Variables|/Script/FreedomFighters.LandVehicle|GetHealthComp (Utilities|Array|Get(acopy) _outactors_3))))
        (if (Math|Random|RandomBool)
          (LocalVariables|SetSpawnLoc (.RandomLocation (AI|Navigation|GetRandomReachablePointinRadius (Transformation|GetSocketLocation (Variables|/Script/FreedomFighters.LandVehicle|GetMeshComp (Utilities|Array|Get(acopy) _outactors_2)) "back_board") 1e+03 0 0)) :!label _label)
          (else
            (LocalVariables|SetSpawnLoc (.RandomLocation (AI|Navigation|GetRandomReachablePointinRadius (Transformation|GetSocketLocation (Variables|/Script/FreedomFighters.LandVehicle|GetMeshComp (Utilities|Array|Get(acopy) _outactors_3)) "back_board") 1e+03 0 0)) :!label _label_2)))
        (bind _groundpoint (CallFunction|GetGroundPoint (LocalVariables|GetSpawnLoc)))
        (bind _returnvalue (Game|SpawnActorfromClass "/Game/_CODFF/Blueprints/Characters/Airborne_BP.Airborne_BP_C" (Math|Transform|MakeTransform _groundpoint "0, 0, 0" "1.000000,1.000000,1.000000") "AdjustIfPossibleButAlwaysSpawn" 0 0))
        (Class|TargetPointComponent|SetPoint (Actor|GetComponentbyClass _array_element "/Script/FreedomFighters.TargetPointComponent") _returnvalue)
        (Utilities|Array|Add (LocalVariables|GetAIMovementComps) (Actor|GetComponentbyClass (AI|GetAIController _returnvalue) "/Script/FreedomFighters.AIMovementComponent"))
        (Utilities|Array|Add (LocalVariables|GetPositions) (Transformation|GetActorLocation (Components|GetOwner (Actor|GetComponentbyClass _array_element "/Script/FreedomFighters.TargetPointComponent"))))
        (elif (Variables|/Script/FreedomFighters.HealthComponent|GetisAlive (Variables|/Script/FreedomFighters.LandVehicle|GetHealthComp (Utilities|Array|Get(acopy) _outactors_2)))
          (goto _label)
          (elif (Variables|/Script/FreedomFighters.HealthComponent|GetisAlive (Variables|/Script/FreedomFighters.LandVehicle|GetHealthComp (Utilities|Array|Get(acopy) _outactors_3)))
            (goto _label_2))))))
  (return (LocalVariables|GetPositions) (LocalVariables|GetAIMovementComps)))

(fn GetMovementPoints
  (params (Tag :type Name))
  (bind _outactors (Actor|GetAllActorswithTag Tag))
  (for _array_element _outactors
    _))

(fn GetGroundPoint0
  (params (Start :type Vector))
  (return (+ Start "0, 0,500.000000")))