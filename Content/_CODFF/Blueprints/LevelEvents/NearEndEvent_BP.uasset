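; NearEndEvent_BP is a level event trigger that starts the near-end music when the player enters its box.
; On overlap it checks that the actor is player character 0, then destroys the box component so it cannot fire again.
; It then casts the game state to GameStateBaseCustom and passes its NearEndMusic to PlayMusic.
; A second IsPlayer function is an unused stub that returns false.
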(event OnComponentBeginOverlap(Box)
  (params (OverlappedComponent :type Primitive%20Component%20Object%20Reference) (OtherActor :type Actor%20Object%20Reference) (OtherComp :type Primitive%20Component%20Object%20Reference) (OtherBodyIndex :type Integer) (bFromSweep :type Boolean) (SweepResult :type Hit%20Result%20Structure%20%28by%20ref%29))
  (if (CallFunction|IsPlayer0 OtherActor)
    (Components|DestroyComponent (Variables|Default|GetBox))
    (bind _asgame_state_base_custom (Utilities|Casting|CastToGameStateBaseCustom (Game|GetGameState)))
    (Class|GameStateBaseCustom|PlayMusic _asgame_state_base_custom (Variables|/Script/FreedomFighters.GameStateBaseCustom|GetNearEndMusic _asgame_state_base_custom))))

(fn ConstructionScript)

(fn IsPlayer
  (params (Actor :type Actor%20Object%20Reference))
  (return false))

(fn IsPlayer0
  (params (Actor :type Actor%20Object%20Reference))
  (return (== Actor (Game|GetPlayerCharacter 0))))