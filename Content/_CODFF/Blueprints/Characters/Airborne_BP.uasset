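; Airborne soldier character Blueprint that randomizes its appearance when play begins.
; A random three-way pick selects the standard shotgun body materials with head A, the red variant with head B or C, or head D alone with materials untouched.
; It swaps upper body and pants materials on the Mesh and sets the skeletal mesh on a separate Head component.
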(event EventBeginPlay
  (bind _head (Variables|Default|GetHead))
  (bind _mesh (Variables|Character|GetMesh))
  (bind _mesh_2 (Variables|Character|GetMesh))
  (switch int (Math|Random|RandomInteger 3)
    (:Default
      (Rendering|Material|SetMaterial _mesh_2 0 "/Game/_CODFF/Models/Characters/COD/Airborne_Russian/Body/B/Materials/mtl_h2_airborne_body_upperbody_shotgun_red.mtl_h2_airborne_body_upperbody_shotgun_red" :!label _label)
      (Rendering|Material|SetMaterial _mesh 3 "/Game/_CODFF/Models/Characters/COD/Airborne_Russian/Body/B/Materials/mtl_h2_airborne_body_pants_shotgun_red.mtl_h2_airborne_body_pants_shotgun_red")
      (switch int (Math|Random|RandomInteger 2)
        (:Default
          (Class|SkinnedMeshComponent|SetSkeletalMesh _head "/Game/_CODFF/Models/Characters/COD/Airborne_Russian/Heads/C/head_airborne_c_LOD0.head_airborne_c_LOD0" true :!label _label_2))
        (:0
          (Class|SkinnedMeshComponent|SetSkeletalMesh _head "/Game/_CODFF/Models/Characters/COD/Airborne_Russian/Heads/B/head_airborne_b.head_airborne_b" true))
        (:1
          (goto _label_2))))
    (:0
      (Rendering|Material|SetMaterial _mesh_2 0 "/Game/_CODFF/Models/Characters/COD/Airborne_Russian/Body/A/Materials/mtl_h2_airborne_body_upperbody_shotgun.mtl_h2_airborne_body_upperbody_shotgun")
      (Rendering|Material|SetMaterial _mesh 3 "/Game/_CODFF/Models/Characters/COD/Airborne_Russian/Body/A/Materials/mtl_h2_airborne_body_pants_shotgun.mtl_h2_airborne_body_pants_shotgun")
      (Class|SkinnedMeshComponent|SetSkeletalMesh (Variables|Default|GetHead) "/Game/_CODFF/Models/Characters/COD/Airborne_Russian/Heads/A/head_airborne_a.head_airborne_a" true))
    (:1
      (goto _label))
    (:2
      (Class|SkinnedMeshComponent|SetSkeletalMesh (Variables|Default|GetHead) "/Game/_CODFF/Models/Characters/COD/Airborne_Russian/Heads/D/head_airborne_d.head_airborne_d" true))))

(fn ConstructionScript)