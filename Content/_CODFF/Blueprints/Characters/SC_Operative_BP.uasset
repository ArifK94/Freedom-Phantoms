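; SC_Operative_BP is an operative character Blueprint that randomizes its head appearance when play begins.
; A first coin flip either keeps the default grey-helmet head or swaps to an alternate green-helmet mesh and removes the shades.
; Further coin flips can invert the helmet color through a material override and, on the default head only, destroy the shades component.
; The construction script is empty, so variation appears only at runtime.
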(event EventBeginPlay
  (switch int (Math|Random|RandomInteger 2)
    (:0
      ;[1 1 1] Stay with the grey helmet - randomly set material to green - randomly choose to wear the glasses
      (switch int (Math|Random|RandomInteger 2)
        (:Default
          _)
        (:0
          (Rendering|Material|SetMaterial (Variables|Default|Gethead_shadow_co_c) 2 "/Game/_CODFF/Models/Characters/COD/ShadowCompany/Helmet/helmet_shadow_green.helmet_shadow_green"))
        (:1
          _))
      (switch int (Math|Random|RandomInteger 2)
        (:0
          (Components|DestroyComponent (Variables|Default|GetShades)))))
    (:1
      ;[0.1099 0.2448 0.05863] Swtich to green helmet - remove glasses - randomly choose helmet material to grey
      (Components|DestroyComponent (Variables|Default|GetShades))
      (Class|SkinnedMeshComponent|SetSkeletalMesh (Variables|Default|Gethead_shadow_co_c) "/Game/_CODFF/Models/Characters/COD/ShadowCompany/Head/head_shadow_co_b/head_shadow_co_b.head_shadow_co_b" false)
      (switch int (Math|Random|RandomInteger 2)
        (:0
          (Rendering|Material|SetMaterial (Variables|Default|Gethead_shadow_co_c) 0 "/Game/_CODFF/Models/Characters/COD/ShadowCompany/Helmet/helmet_shadow_grey.helmet_shadow_grey"))))))

(fn ConstructionScript)