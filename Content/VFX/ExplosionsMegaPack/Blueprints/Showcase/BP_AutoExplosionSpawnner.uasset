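; BP_AutoExplosionSpawnner is a showcase actor that repeatedly spawns an explosion effect at a configurable location.
; SpawnExplossion spawns either a particle emitter or, when a grenade class is set, a BP_PyroGrenade with deactivated projectile movement and overridden blast and fire effects.
; It then resets three LEDs to red, runs Charge to light them green in sequence, and calls itself again after SpawnDelay.
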(event Custom|SpawnExplossion
  (bind _pyrogrenade (Variables|Customize|GetPyroGrenade))
  (bind _explosionspawnlocation (Variables|Default|GetExplosionSpawnLocation))
  ;[1 1 1] First we check if it should spawn an Particle Emitter or a Blueprint
  (if (Utilities|IsValidClass (.GrenadeActor (Utilities|Struct|BreakPyroGrenade (Variables|Customize|GetPyroGrenade))))
    ;[1 1 1] Here we spawn the custom blueprint (used for the Pyro Explosions)
    (bind _returnvalue (Game|SpawnActorfromClass (.grenadeactor (Variables|Customize|GetPyroGrenade)) (Transformation|GetWorldTransform _explosionspawnlocation) "AlwaysSpawn" 0 0))
    ;[1 1 1] Here we cast the blueprint in order to customize it so we can spawn different variations
    (bind _asbp_pyro_grenade (Utilities|Casting|CastToBP_PyroGrenade _returnvalue))
    (Utilities|FlowControl|Sequence
      (:then_0
        (Components|Activation|Deactivate (Variables|/Game/VFX/ExplosionsMegaPack/Blueprints/Pyro/BP_PyroGrenade.BP_PyroGrenade_C|GetProjectileMovement _asbp_pyro_grenade)))
      (:then_1
        (Variables|/Game/VFX/ExplosionsMegaPack/Blueprints/Pyro/BP_PyroGrenade.BP_PyroGrenade_C|SetPfx_Explosion _asbp_pyro_grenade (.pfxblast _pyrogrenade)))
      (:then_2
        (Variables|/Game/VFX/ExplosionsMegaPack/Blueprints/Pyro/BP_PyroGrenade.BP_PyroGrenade_C|SetPfx_FireSmall _asbp_pyro_grenade (.pfxfiresmall _pyrogrenade)))
      (:then_3
        (Variables|/Game/VFX/ExplosionsMegaPack/Blueprints/Pyro/BP_PyroGrenade.BP_PyroGrenade_C|SetPfx_FireMedium _asbp_pyro_grenade (.pfxfiremedium _pyrogrenade)))
      (:then_4
        (Variables|/Game/VFX/ExplosionsMegaPack/Blueprints/Pyro/BP_PyroGrenade.BP_PyroGrenade_C|SetPfx_FireLarge _asbp_pyro_grenade (.pfxfirelarge _pyrogrenade)))
      (:then_5
        ;[1 1 1] After the effect is spawnned we turn off the LED's
        (Rendering|Material|SetMaterial (Variables|Default|GetLED%2001) 0 "/Game/VFX/ExplosionsMegaPack/Materials/Showcase/M_Showcase_LED_Red.M_Showcase_LED_Red" :!label _label)
        (Rendering|Components|Light|SetIntensity (Variables|Default|GetPointLight_01) 0.0)
        ;[1 1 1] This controls the LED's during charging
        (CallFunction|Charge)
        ;[1 1 1] The actual charging / delay
        (Utilities|FlowControl|Delay (Variables|Customize|GetSpawn%20Delay))
        ;[1 1 1] After the delay we spawn a new instance of the effect
        (CallFunction|SpawnExplossion)))
    (else
      ;[1 1 1] Here we spawn the particle emitter at the custom location
      (Effects|SpawnEmitteratLocation (Variables|Customize|GetPFX%20To%20Spawn) (Transformation|GetWorldLocation _explosionspawnlocation))
      (goto _label))))

(event Custom|Charge
  (bind _spawn_delay (Variables|Customize|GetSpawn%20Delay))
  (bind _returnvalue (/ _spawn_delay 3.2))
  ;[1 1 1] This controls the LED's
  ;[1 1 1] After, we turn On each LED using the same delay between each
  (Utilities|FlowControl|Delay _returnvalue)
  (Utilities|FlowControl|Sequence
    (:then_0
      (Rendering|Material|SetMaterial (Variables|Default|GetLED%2001) 0 "/Game/VFX/ExplosionsMegaPack/Materials/Showcase/M_Showcase_LED_Green.M_Showcase_LED_Green")
      (Utilities|FlowControl|Delay _returnvalue)
      (Utilities|FlowControl|Sequence
        (:then_0
          (Rendering|Material|SetMaterial (Variables|Default|GetLED%2002) 0 "/Game/VFX/ExplosionsMegaPack/Materials/Showcase/M_Showcase_LED_Green.M_Showcase_LED_Green")
          (Utilities|FlowControl|Delay _returnvalue)
          (Utilities|FlowControl|Sequence
            (:then_0
              (Rendering|Material|SetMaterial (Variables|Default|GetLED%2003) 0 "/Game/VFX/ExplosionsMegaPack/Materials/Showcase/M_Showcase_LED_Green.M_Showcase_LED_Green"))
            (:then_1
              (Rendering|Components|Light|SetIntensity (Variables|Default|GetPointLight_03) 1e+02))))
        (:then_1
          (Rendering|Components|Light|SetIntensity (Variables|Default|GetPointLight_02) 1e+02))))
    (:then_1
      (Rendering|Components|Light|SetIntensity (Variables|Default|GetPointLight_01) 1e+02))))

(event EventBeginPlay
  ;[1 1 1] We begin the spawnning loop when the game starts
  (CallFunction|Charge)
  (Utilities|FlowControl|Delay (Variables|Customize|GetSpawn%20Delay))
  (CallFunction|SpawnExplossion))

(fn ConstructionScript
  (Transformation|SetRelativeLocation (Variables|Default|GetExplosionSpawnLocation) (Variables|Customize|GetSpawnLocation) false false))