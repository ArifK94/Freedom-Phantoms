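; Showcase trigger volume that lets the player throw pyro grenades with the left mouse button while inside it.
; Box overlaps with a DefaultPawn enable or disable input and open or close a Gate that the click feeds.
; A DoOnce with a delayed reset throttles spawning to protect performance.
; Each BP_PyroGrenade spawns just below the camera along its view rotation, then receives this actor's explosion and fire effects.
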(event OnComponentBeginOverlap(Box)
  (params (OverlappedComponent :type Primitive%20Component%20Object%20Reference) (OtherActor :type Actor%20Object%20Reference) (OtherComp :type Primitive%20Component%20Object%20Reference) (OtherBodyIndex :type Integer) (bFromSweep :type Boolean) (SweepResult :type Hit%20Result%20Structure%20%28by%20ref%29))
  (bind _returnvalue (Game|GetPlayerCameraManager 0))
  ;[1 1 1] Here we detect if the player entered the trigger zone, and if so we enable the input
  (Utilities|Casting|CastToDefaultPawn OtherActor)
  (Input|EnableInput (Game|GetPlayerController 0))
  ;[1 1 1] Open / Close the gate depending if the player is inside the trigger or not
  (Utilities|FlowControl|Gate true) ; enters at Open
)

(event OnComponentEndOverlap(Box)
  (params (OverlappedComponent :type Primitive%20Component%20Object%20Reference) (OtherActor :type Actor%20Object%20Reference) (OtherComp :type Primitive%20Component%20Object%20Reference) (OtherBodyIndex :type Integer))
  (bind _returnvalue (Game|GetPlayerCameraManager 0))
  ;[1 1 1] Here we detect if the player left the trigger zone and disable the input so that he won't be able to spawn grenades outside
  (Utilities|Casting|CastToDefaultPawn OtherActor)
  (Input|DisableInput (Game|GetPlayerController 0))
  ;[1 1 1] Open / Close the gate depending if the player is inside the trigger or not
  (Utilities|FlowControl|Gate true) ; enters at Close
)

(event Input|MouseEvents|LeftMouseButton
  (params (Key :type Key%20Structure))
  (bind _returnvalue (Game|GetPlayerCameraManager 0))
  ;[1 1 1] On Left Mouse Button we try to spawn
  (:Pressed
    ;[1 1 1] Open / Close the gate depending if the player is inside the trigger or not
    (Utilities|FlowControl|Gate true
      (:Exit
        ;[1 1 1] We use this to prevent spawnning too many Pyro Explosions too fast as this can affect performance
        (Utilities|FlowControl|DoOnce false :!label _label
          (:Completed
            ;[1 1 1] Here we spawn the Pyro Grenader Blueprint
            (bind _returnvalue_2 (Game|SpawnActorfromClass "/Game/VFX/ExplosionsMegaPack/Blueprints/Pyro/BP_PyroGrenade.BP_PyroGrenade_C" (Math|Transform|MakeTransform (- (Camera|GetCameraLocation _returnvalue) "0, 0,25.000000") (Camera|GetCameraRotation _returnvalue) "1,1,1") "Undefined" 0 0))
            ;[1 1 1] We then customize the effect
            (Variables|/Game/VFX/ExplosionsMegaPack/Blueprints/Pyro/BP_PyroGrenade.BP_PyroGrenade_C|SetPfx_Explosion _returnvalue_2 (Variables|Customize|GetPfx_Explosion))
            (Variables|/Game/VFX/ExplosionsMegaPack/Blueprints/Pyro/BP_PyroGrenade.BP_PyroGrenade_C|SetPfx_FireLarge _returnvalue_2 (Variables|Customize|GetPfx_FireLarge))
            (Variables|/Game/VFX/ExplosionsMegaPack/Blueprints/Pyro/BP_PyroGrenade.BP_PyroGrenade_C|SetPfx_FireMedium _returnvalue_2 (Variables|Customize|GetPfx_FireMedium))
            (Variables|/Game/VFX/ExplosionsMegaPack/Blueprints/Pyro/BP_PyroGrenade.BP_PyroGrenade_C|SetPfx_FireSmall _returnvalue_2 (Variables|Customize|GetPfx_FireSmall))
            ;[1 1 1] This determines how fast can we spawn this effect
            (Utilities|FlowControl|Delay 1.0)
            (goto _label Reset)))))))

(fn ConstructionScript)