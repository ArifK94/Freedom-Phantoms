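; Showcase trigger zone that lets the player fire explosion grenades with the left mouse button while inside it.
; Box overlap by a DefaultPawn toggles input and a Gate, so clicks spawn a grenade slightly below the camera, facing the view direction.
; The Construction Script picks the Simple or Advanced grenade class from the Advanced flag.
; Each spawned grenade receives the radial emitter, and the Advanced one also gets a directional emitter.
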(event OnComponentBeginOverlap(Box)
  (params (OverlappedComponent :type Primitive%20Component%20Object%20Reference) (OtherActor :type Actor%20Object%20Reference) (OtherComp :type Primitive%20Component%20Object%20Reference) (OtherBodyIndex :type Integer) (bFromSweep :type Boolean) (SweepResult :type Hit%20Result%20Structure%20%28by%20ref%29))
  (bind _returnvalue (Game|GetPlayerCameraManager 0))
  ;[1 1 1] Here we detect if the player entered the trigger zone, and if so we enable the input
  (Utilities|Casting|CastToDefaultPawn OtherActor)
  (Input|EnableInput (Game|GetPlayerController 0))
  ;[1 1 1] Open / Close the gate depending if the player is inside the trigger or not
  (Utilities|FlowControl|Gate true) ; enters at Open
)

(event OnComponentEndOverlap(Box)
  (params (OverlappedComponent :type Primitive%20Component%20Object%20Reference) (OtherActor :type Actor%20Object%20Reference) (OtherComp :type Primitive%20Component%20Object%20Reference) (OtherBodyIndex :type Integer))
  (bind _returnvalue (Game|GetPlayerCameraManager 0))
  ;[1 1 1] Here we detect if the player left the trigger zone and disable the input so that he won't be able to spawn grenades outside
  (Utilities|Casting|CastToDefaultPawn OtherActor)
  (Input|DisableInput (Game|GetPlayerController 0))
  ;[1 1 1] Open / Close the gate depending if the player is inside the trigger or not
  (Utilities|FlowControl|Gate true) ; enters at Close
)

(event Input|MouseEvents|LeftMouseButton
  (params (Key :type Key%20Structure))
  (bind _returnvalue (Game|GetPlayerCameraManager 0))
  ;[1 1 1] On Left Mouse Button we try to spawn
  (:Pressed
    ;[1 1 1] Open / Close the gate depending if the player is inside the trigger or not
    (Utilities|FlowControl|Gate true
      (:Exit
        ;[1 1 1] Here we spawn the actor. "Actor" is set in the Construction scriopt and can be either the Simple or the Advanced Grenade.
        (bind _returnvalue_2 (Game|SpawnActorfromClass (Variables|Customize|GetActorToSpawn) (Math|Transform|MakeTransform (- (Camera|GetCameraLocation _returnvalue) "0, 0,25.000000") (Camera|GetCameraRotation _returnvalue) "1,1,1") "Undefined" 0 0))
        ;[1 1 1] Here we customize the Simple Grenade
        (bind _asbp_grenade_simple (Utilities|Casting|CastToBP_Grenade_Simple _returnvalue_2)
          (:then
            (Variables|/Game/VFX/ExplosionsMegaPack/Blueprints/Showcase/BP_Grenade_Simple.BP_Grenade_Simple_C|SetEmitterToSpawn _asbp_grenade_simple (Variables|Customize|GetEmitterToSpawn_Radial)))
          (:CastFailed
            ;[1 1 1] Here we customize the Advanced Grenade
            (bind _asbp_grenade_advanced (Utilities|Casting|CastToBP_Grenade_Advanced _returnvalue_2))
            (Variables|/Game/VFX/ExplosionsMegaPack/Blueprints/Showcase/BP_Grenade_Advanced.BP_Grenade_Advanced_C|SetEmitterToSpawnDirectional _asbp_grenade_advanced (Variables|Customize|GetEmitterToSpawn_Directional))
            (Variables|/Game/VFX/ExplosionsMegaPack/Blueprints/Showcase/BP_Grenade_Advanced.BP_Grenade_Advanced_C|SetEmitterToSpawnRadial _asbp_grenade_advanced (Variables|Customize|GetEmitterToSpawn_Radial))))))))

(fn ConstructionScript
  ;[1 1 1] Defines if the player should spawn a Simple Grenade or an Advanced One
  (if (Variables|Customize|GetAdvanced?)
    (Variables|Customize|SetActorToSpawn "/Game/VFX/ExplosionsMegaPack/Blueprints/Showcase/BP_Grenade_Advanced.BP_Grenade_Advanced_C")
    (else
      (Variables|Customize|SetActorToSpawn "/Game/VFX/ExplosionsMegaPack/Blueprints/Showcase/BP_Grenade_Simple.BP_Grenade_Simple_C"))))