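; Pyro grenade actor that explodes once, on first overlap or after a short fuse, leaving fires on nearby surfaces.
; It spawns the blast and hides its mesh, then fires random line traces within a radius.
; Hits spawn randomly scaled, normal-aligned fire effects, larger nearer the blast, using distance bands over a hard-coded range.
; The stored looping fires are later deactivated one by one before the actor destroys itself.
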(event OnComponentBeginOverlap(CollisionComponent)
  (params (OverlappedComponent :type Primitive%20Component%20Object%20Reference) (OtherActor :type Actor%20Object%20Reference) (OtherComp :type Primitive%20Component%20Object%20Reference) (OtherBodyIndex :type Integer) (bFromSweep :type Boolean) (SweepResult :type Hit%20Result%20Structure%20%28by%20ref%29))
  ;[1 1 1] If the collider overlaps with a prop we trigger the explosion
  ;[1 1 1] This makes sure that the explosion triggers only once
  (Utilities|FlowControl|DoOnce false
    (:Completed
      (CallFunction|Explode))))

(event Custom|Explode
  (bind _returnvalue (Math|Random|RandomFloatinRange 0.8 1.4))
  (bind _returnvalue_2 (Transformation|GetActorLocation))
  (bind _spawnedeffects (Variables|Default|GetSpawnedEffects))
  (bind _index (Variables|Default|GetIndex))
  (Utilities|FlowControl|Sequence
    (:then_0
      ;[1 1 1] First we spawn the main explosion blast
      (Effects|SpawnEmitteratLocation (Variables|Customize|GetPfx_Explosion) (Transformation|GetActorLocation))
      ;[1 1 1] Then we hide the grenade mesh because we can't delete this actor yet
      (Rendering|SetVisibility (Variables|Default|GetStaticMesh) false false))
    (:then_1
      ;[1 1 1] We wait a bit to give the blast time to expand
      (Utilities|FlowControl|Delay 0.1)
      ;[1 1 1] This sets how many times we should test for nearby objects
      (for _index_2 (range 0 (Variables|Customize|GetNumberOfTraces))
        ;[1 1 1] For each time we want to test for close objects we shoot line trace
        (bind (_outhit _returnvalue_3) (Collision|LineTraceForObjects _returnvalue_2 (+ _returnvalue_2 (* (Math|Vector|GetForwardVector (Math|Random|RandomRotator true)) (Variables|Customize|GetRadiusToSpawnFire))) (Variables|Customize|GetObjectType) false 0 (Variables|Customize|GetDebugTrace)))
        ;[1 1 1] If we hit something we continue
        (if _returnvalue_3
          ;[1 1 1] Then depending on the distance we spawn larger or smaller fire effects - the closer to the explosion, the larger the fire
          (if (Math|Float|InRange(Float) (/ (Math|Vector|VectorLength (- (.tracestart _outhit) (.location _outhit))) 5e+02) 0.0 0.33)
            (Variables|Default|SetFireTypeIndex 2)
            ;[1 1 1] We spawn the fire effect at the impact location and aligned to the impact surface normal
            (bind _returnvalue_4 (Effects|SpawnEmitteratLocation (Utilities|Select :Index (Variables|Default|GetFireTypeIndex) :Option%200 (Variables|Customize|GetPfx_FireSmall) :Option%201 (Variables|Customize|GetPfx_FireMedium) :Option%202 (Variables|Customize|GetPfx_FireLarge)) (.location _outhit) (Math|Rotator|CombineRotators (Math|Rotator|MakeRotfromZ (.normal _outhit)) (Math|Vector|RotatorfromAxisandAngle (.normal _outhit) (Math|Random|RandomFloatinRange 0.0 3.6e+02))) :!label _label))
            ;[1 1 1] We randomize the size of the effect
            (Transformation|SetRelativeScale3D _returnvalue_4 (Math|Vector|MakeVector _returnvalue _returnvalue _returnvalue))
            ;[1 1 1] Here we store the spawnned fire effects so that we can turn them off later
            (Utilities|Array|Add (Variables|Default|GetSpawnedEffects) _returnvalue_4)
            (elif (Math|Float|InRange(Float) (/ (Math|Vector|VectorLength (- (.tracestart _outhit) (.location _outhit))) 5e+02) 0.34 0.66)
              (Variables|Default|SetFireTypeIndex 1)
              (goto _label)
              (elif (Math|Float|InRange(Float) (/ (Math|Vector|VectorLength (- (.tracestart _outhit) (.location _outhit))) 5e+02) 0.67 1.0)
                (Variables|Default|SetFireTypeIndex 0)
                (goto _label))))))
      ;[1 1 1] After 5 seconds we start turning off the spawnned fire effects
      ; They are looping so we need to do this manually - in your project you might want to make the fire not to loop
      (Utilities|FlowControl|Delay 5.0)
      ;[1 1 1] We deactivate each spawnned effect every 0.5 seconds then we destroy this actor
      (if (> (Utilities|Array|Length _spawnedeffects) _index) :!label _label_2
        (Components|Activation|Deactivate (Utilities|Array|Get(acopy) _spawnedeffects _index))
        (Math|Integer|IncrementInt (Variables|Default|GetIndex)
          (:%20%20
            (Utilities|FlowControl|Delay 0.5)
            (goto _label_2)))
        (else
          (Actor|DestroyActor))))))

(event EventBeginPlay
  ;[1 1 1] In case that the grenade doesn't collide with anything for 0.75 seconds we trigger the explosion
  (Utilities|FlowControl|Delay 0.75)
  ;[1 1 1] This makes sure that the explosion triggers only once
  (Utilities|FlowControl|DoOnce false
    (:Completed
      (CallFunction|Explode))))

(fn ConstructionScript)